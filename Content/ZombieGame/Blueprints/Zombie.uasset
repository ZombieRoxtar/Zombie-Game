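; Zombie enemy that wanders between random reachable points, then chases and attacks the player once PawnSensing spots them.
; Reaching the player opens a timed attack window where an AttackArea overlap deals damage at most once, then the chase repeats.
; Projectile overlaps reduce health and send it toward the player without setting SeenPlayer.
; At zero health the mesh ragdolls and a KillPopup widget appears.
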(event OnSeePawn(PawnSensing)
  (params (Pawn :type Pawn%20Object%20Reference))
  ;[1 1 1] Sense Player
  (bind _asperson_character (Utilities|Casting|CastToPersonCharacter Pawn))
  (Variables|Default|SetSeen%20Player true)
  (AI|AIMoveTo self "0, 0, 0" _asperson_character 5.0 false :!label _label
    (:OnSuccess
      (if (not (Variables|Default|GetIs%20Attacking))
        (Variables|Default|SetIs%20Attacking true)
        (Utilities|FlowControl|Delay 2.3)
        (Variables|Default|SetIs%20Attacking false)
        (Variables|Default|SetAlready%20Hit false)
        (goto _label)))))

(event OnComponentBeginOverlap(AttackArea)
  (params (OverlappedComponent :type Primitive%20Component%20Object%20Reference) (OtherActor :type Actor%20Object%20Reference) (OtherComp :type Primitive%20Component%20Object%20Reference) (OtherBodyIndex :type Integer) (bFromSweep :type Boolean) (SweepResult :type Hit%20Result%20Structure%20%28by%20ref%29))
  ;[1 1 1] Deal Damage
  (bind _asperson_character (Utilities|Casting|CastToPersonCharacter OtherActor))
  (if (Variables|Default|GetIs%20Attacking)
    (if (not (Variables|Default|GetAlready%20Hit))
      (Default|TakeDamage _asperson_character 0.2)
      (Variables|Default|SetAlready%20Hit true))))

(event Custom|Chase%20Player
  ;[1 1 1] Chase Player
  (bind _asperson_character (Utilities|Casting|CastToPersonCharacter (Game|GetPlayerCharacter 0)))
  (AI|AIMoveTo self "0, 0, 0" _asperson_character 5.0 false))

(event EventBeginPlay
  ;[1 1 1] Start Wandering
  (AI|AIMoveTo self (.RandomLocation (AI|Navigation|GetRandomReachablePointinRadius (Transformation|GetActorLocation) 1e+04 0 0)) 0 5.0 true :!label _label
    (:OnSuccess
      _)
    (:OnFail
      _))
  (if (not (Variables|Default|GetSeen%20Player))
    (Utilities|FlowControl|Delay 1.0)
    (goto _label)))

(event Collision|EventActorBeginOverlap
  (params (OtherActor :type Actor%20Object%20Reference))
  ;[1 1 1] Take Damage
  (Utilities|Casting|CastToProjectileBase OtherActor)
  (CallFunction|TakeDamage 0.1))

(event EventTick
  (params (DeltaSeconds :type Float%20%28single-precision%29)))

(fn ConstructionScript)

(fn TakeDamage
  (params (Damage :type Float%20%28single-precision%29))
  (if (not (Variables|Default|GetIs%20Dead))
    (bind _output_get (Variables|Default|SetHealth (- (Variables|Default|GetHealth) Damage)))
    (if (<= _output_get 0.0)
      (Variables|Default|SetIs%20Dead true)
      (Physics|SetSimulatePhysics (Variables|Character|GetMesh) true)
      (bind _returnvalue (UserInterface|CreateWidget "/Game/ZombieGame/Blueprints/HUD/KillPopup.KillPopup_C"))
      (Default|SetDeadee _returnvalue "zombie")
      (UserInterface|Viewport|AddtoViewport _returnvalue 0)
      (else
        (CallFunction|ChasePlayer)))))