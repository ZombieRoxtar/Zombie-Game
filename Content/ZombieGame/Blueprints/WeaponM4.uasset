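; WeaponM4 is the M4 rifle weapon Blueprint for the zombie game, handling firing and reloading.
; Fire spawns a ProjectileBase at the Muzzle socket, decrements Clip, and attaches a muzzle flash and gunshot sound to the skeletal mesh.
; Reload returns leftover rounds to the player PersonCharacter's ammo pool, then refills Clip up to ClipSize or whatever the pool holds, skipping when already full.
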(event Custom|Fire
  (bind _skeletalmesh (Variables|Default|GetSkeletalMesh))
  (Game|SpawnActorfromClass "/Game/ZombieGame/Blueprints/ProjectileBase.ProjectileBase_C" (Transformation|GetSocketTransform _skeletalmesh "Muzzle" "RTS_World") "Undefined" 0 0)
  (Variables|Default|SetClip (- (Variables|Default|GetClip) 1))
  (Effects|SpawnEmitterAttached "/Game/InfinityBladeEffects/Effects/FX_Monsters/FX_Monster_Chicken/P_ChickenMaster_MuzzleFlash_01.P_ChickenMaster_MuzzleFlash_01" _skeletalmesh "Muzzle" "0, 0, 0" "0, 0, 0" "0.250000,0.250000,0.250000")
  (Audio|SpawnSoundAttached "/Game/FPSassets/Effects/M4A1_Single.M4A1_Single" _skeletalmesh "None" "0, 0, 0" "0, 0, 0" "KeepRelativeOffset" false 1.0 1.0 0.0 0 0))

(event EventBeginPlay)

(event Collision|EventActorBeginOverlap
  (params (OtherActor :type Actor%20Object%20Reference)))

(event EventTick
  (params (DeltaSeconds :type Float%20%28single-precision%29)))

(fn ConstructionScript)

(fn Reload
  (bind _clipsize (Variables|Default|GetClipSize))
  (bind _asperson_character (Utilities|Casting|CastToPersonCharacter (Game|GetPlayerCharacter 0)))
  (if (!= (Variables|Default|GetClip) _clipsize) ; Don't reload if it's full.
    (Default|AddAmmo _asperson_character (Variables|Default|GetClip)) ; Put the current amt into the pool.
    (if (< (Variables|/Game/ZombieGame/Blueprints/PersonCharacter.PersonCharacter_C|GetAmmo _asperson_character) _clipsize)
      (bind _output_get (Variables|Default|SetClip (Variables|/Game/ZombieGame/Blueprints/PersonCharacter.PersonCharacter_C|GetAmmo _asperson_character)))
      (Default|RemoveAmmo _asperson_character _output_get)
      (else
        (bind _output_get_2 (Variables|Default|SetClip _clipsize))
        (Default|RemoveAmmo _asperson_character _output_get_2)))))