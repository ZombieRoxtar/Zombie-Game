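; PersonGameMode is a game mode Blueprint that enforces a play time limit in the zombie game.
; Tick runs through a one-second Delay, then compares a nonzero TimeLimit with the rounded game time in seconds.
; When time is up, it pauses the game, calls ShowPausedBox on the player's PersonCharacter, and zeroes TimeLimit so the check does not fire again.
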(event EventTick
  (params (DeltaSeconds :type Float%20%28single-precision%29))
  (Utilities|FlowControl|Delay 1.0)
  (if (>= (Variables|Default|GetTimeLimit) 1)
    (if (<= (Variables|Default|GetTimeLimit) (Math|Float|Round (Utilities|Time|GetGameTimeinSeconds)))
      (bind _asperson_character (Utilities|Casting|CastToPersonCharacter (Game|GetPlayerCharacter 0)))
      (Game|SetGamePaused true)
      (Default|ShowPausedBox _asperson_character)
      (Variables|Default|SetTimeLimit 0))))

(fn ConstructionScript)