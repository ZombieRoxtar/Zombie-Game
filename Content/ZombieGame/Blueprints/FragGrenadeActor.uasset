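; Thrown frag grenade actor that damages zombies in a radius when it explodes.
; On spawn it launches its static mesh along the player controller's aim, then waits a short fuse delay.
; It then plays explosion effects and sound, calls TakeDamage on every Zombie overlapping its sphere, and destroys itself.
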(event EventBeginPlay
  (bind _staticmesh (Variables|Default|GetStaticMesh))
  (Physics|AddImpulse _staticmesh (* (Math|Rotator|GetRotationXVector (Pawn|GetControlRotation (Game|GetPlayerController 0) :!class /Script/Engine.Controller)) "1000.000000,1000.000000,1000.000000") "None" false)
  (Utilities|FlowControl|Delay 2.0)
  (Effects|SpawnEmitterAttached "/Game/StarterContent/Particles/P_Explosion.P_Explosion" _staticmesh "None" "0, 0, 0" "0, 0, 0" "30.000000,30.000000,30.000000")
  (Audio|SpawnSoundatLocation "/Game/StarterContent/Audio/Explosion_Cue.Explosion_Cue" (Transformation|GetWorldLocation _staticmesh) "0, 0, 0" 1.0 1.0 0.0 0 0)
  (for _array_element (Collision|GetOverlappingActors (Variables|Default|GetSphere) "/Game/ZombieGame/Blueprints/Zombie.Zombie_C" :!class /Script/Engine.PrimitiveComponent)
    (bind _aszombie (Utilities|Casting|CastToZombie _array_element))
    (Default|TakeDamage _aszombie 1.0))
  (Actor|DestroyActor))

(event Collision|EventActorBeginOverlap
  (params (OtherActor :type Actor%20Object%20Reference)))

(event EventTick
  (params (DeltaSeconds :type Float%20%28single-precision%29)))

(fn ConstructionScript)