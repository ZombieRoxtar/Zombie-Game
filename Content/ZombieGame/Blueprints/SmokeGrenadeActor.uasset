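; Smoke grenade actor that is thrown along the first player's view direction and goes off after a short fuse.
; On BeginPlay it applies an impulse to its static mesh along the player controller's control rotation, then waits on a delay.
; It then spawns a scaled smoke emitter and explosion sound at the mesh location, immediately destroys that emitter component, and destroys itself.
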(event EventBeginPlay
  (bind _staticmesh (Variables|Default|GetStaticMesh))
  (bind _returnvalue (Transformation|GetWorldLocation _staticmesh))
  (Physics|AddImpulse _staticmesh (* (Math|Rotator|GetRotationXVector (Pawn|GetControlRotation (Game|GetPlayerController 0) :!class /Script/Engine.Controller)) "1000.000000,1000.000000,1000.000000") "None" false)
  (Utilities|FlowControl|Delay 2.0)
  (bind _returnvalue_2 (Effects|SpawnEmitteratLocation "/Game/StarterContent/Particles/P_Smoke.P_Smoke" _returnvalue "0, 0, 0" "5.000000,5.000000,5.000000"))
  (Audio|SpawnSoundatLocation "/Game/StarterContent/Audio/Explosion_Cue.Explosion_Cue" _returnvalue "0, 0, 0" 1.0 1.0 0.0 0 0)
  (Components|DestroyComponent _returnvalue_2)
  (Actor|DestroyActor))

(event Collision|EventActorBeginOverlap
  (params (OtherActor :type Actor%20Object%20Reference)))

(event EventTick
  (params (DeltaSeconds :type Float%20%28single-precision%29)))

(fn ConstructionScript)